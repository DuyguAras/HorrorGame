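; A single keypad button actor that reports clicks to its owning keypad.
; Hovering swaps the button mesh to a chrome material and leaving it, or a ResetButtons call, restores gold.
; Clicking passes the button's text value plus confirm and backspace flags to the referenced keypad's EnteredButton, and the construction script shows that value on the button's number text.
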(event OnBeginCursorOver(Button)
  (params (TouchedComponent :type Primitive%20Component%20Object%20Reference))
  ;[1 1 1] Mouse Cursor
  (Rendering|Material|SetMaterial (Variables|Default|GetButton) 0 "/Game/StarterContent/Materials/M_Metal_Chrome.M_Metal_Chrome"))

(event OnEndCursorOver(Button)
  (params (TouchedComponent :type Primitive%20Component%20Object%20Reference))
  ;[1 1 1] Mouse Cursor
  (Rendering|Material|SetMaterial (Variables|Default|GetButton) 0 "/Game/StarterContent/Materials/M_Metal_Gold.M_Metal_Gold"))

(event OnClicked(Button)
  (params (TouchedComponent :type Primitive%20Component%20Object%20Reference) (ButtonPressed :type Key%20Structure :default "None"))
  ;[1 1 1] On Clicked Event
  (Default|EnteredButton (Variables|Default|GetKeypadRef) (Variables|Default|GetNoText) (Variables|Default|GetConfirmedButton) (Variables|Default|GetBackspacedButton)))

(event Custom|ResetButtons
  ;[1 1 1] Mouse Cursor
  (Rendering|Material|SetMaterial (Variables|Default|GetButton) 0 "/Game/StarterContent/Materials/M_Metal_Gold.M_Metal_Gold"))

(fn ConstructionScript
  (Rendering|Components|TextRender|SetText (Variables|Default|GetButtonNumber) (Variables|Default|GetNoText)))