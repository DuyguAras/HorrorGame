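; Interactable keypad puzzle that unlocks the BP_LockedBox and BP_Door found in the level when the right code is entered.
; Interacting blends the view to the keypad camera, enables mouse clicks and hands a self reference to the child-actor BP_KeypadButtons.
; Button input types, backspaces or confirms the text compared against KeypadCode.
; A wrong code resets entry after a delay; a correct one restores the player camera and disables further interaction.
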(event Custom|OnInteracted
  (bind _returnvalue (Game|GetPlayerController 0))
  ;[1 1 1] The Event When Buttons Are Pressed
  (Variables|/Game/ThirdPersonBP/Blueprints/ThirdPersonCharacter.ThirdPersonCharacter_C|SetCurrentPlayerState (Variables|Default|GetPlayerRef) "NewEnumerator1")
  (Game|Player|SetViewTargetwithBlend (Game|GetPlayerController 0) (Components|GetOwner (Variables|Default|GetCamera)) 0.4 "VTBlend_Linear" 0.0 false)
  (bind _output_get (Variables|/Script/Engine.PlayerController|SetbShowMouseCursor _returnvalue true))
  (bind _output_get_2 (Variables|/Script/Engine.PlayerController|SetbEnableClickEvents _returnvalue _output_get))
  (Variables|/Script/Engine.PlayerController|SetbEnableMouseOverEvents _returnvalue _output_get_2)
  (Rendering|Components|TextRender|SetText (Variables|Default|GetEnteredCodeText) (Utilities|Text|MakeLiteralText (Utilities|Text|ToText(String) (Utilities|String|GetSubstring (Utilities|String|MakeLiteralString "____") 0 (Utilities|String|Len (Variables|Default|GetKeypadCode))))))
  (bind _output_get_3 (Variables|Default|SetButtonArray (Utilities|Array|MakeArray (Variables|Default|GetBP_KeypadButton0) (Variables|Default|GetBP_KeypadButton1) (Variables|Default|GetBP_KeypadButton2) (Variables|Default|GetBP_KeypadButton3) (Variables|Default|GetBP_KeypadButton4) (Variables|Default|GetBP_KeypadButton5) (Variables|Default|GetBP_KeypadButton6) (Variables|Default|GetBP_KeypadButton7) (Variables|Default|GetBP_KeypadButton8) (Variables|Default|GetBP_KeypadButton9) (Variables|Default|GetBP_KeypadButtonBack) (Variables|Default|GetBP_KeypadButtonForward))))
  (for _array_element _output_get_3
    (bind _asbp_keypad_button (Utilities|Casting|CastToBP_KeypadButton (Variables|/Script/Engine.ChildActorComponent|GetChildActor _array_element)))
    (Variables|/Game/Objects/BP_KeypadButton.BP_KeypadButton_C|SetKeypadRef _asbp_keypad_button self)))

(event Custom|Initiate
  (bind _returnvalue (Game|GetPlayerController 0))
  ;[1 1 1] The Event When Buttons Are Pressed
  (bind _output_get (Variables|/Script/Engine.PlayerController|SetbShowMouseCursor _returnvalue true))
  (bind _output_get_2 (Variables|/Script/Engine.PlayerController|SetbEnableClickEvents _returnvalue _output_get))
  (Variables|/Script/Engine.PlayerController|SetbEnableMouseOverEvents _returnvalue _output_get_2)
  (Rendering|Components|TextRender|SetText (Variables|Default|GetEnteredCodeText) (Utilities|Text|MakeLiteralText (Utilities|Text|ToText(String) (Utilities|String|GetSubstring (Utilities|String|MakeLiteralString "____") 0 (Utilities|String|Len (Variables|Default|GetKeypadCode))))))
  (bind _output_get_3 (Variables|Default|SetButtonArray (Utilities|Array|MakeArray (Variables|Default|GetBP_KeypadButton0) (Variables|Default|GetBP_KeypadButton1) (Variables|Default|GetBP_KeypadButton2) (Variables|Default|GetBP_KeypadButton3) (Variables|Default|GetBP_KeypadButton4) (Variables|Default|GetBP_KeypadButton5) (Variables|Default|GetBP_KeypadButton6) (Variables|Default|GetBP_KeypadButton7) (Variables|Default|GetBP_KeypadButton8) (Variables|Default|GetBP_KeypadButton9) (Variables|Default|GetBP_KeypadButtonBack) (Variables|Default|GetBP_KeypadButtonForward))))
  (for _array_element _output_get_3
    (bind _asbp_keypad_button (Utilities|Casting|CastToBP_KeypadButton (Variables|/Script/Engine.ChildActorComponent|GetChildActor _array_element)))
    (Variables|/Game/Objects/BP_KeypadButton.BP_KeypadButton_C|SetKeypadRef _asbp_keypad_button self)))

(event Custom|Backspace
  (bind _enteredcodetext (Variables|Default|GetEnteredCodeText))
  (bind _text (Variables|/Script/Engine.TextRenderComponent|GetText _enteredcodetext))
  (bind _returnvalue (Utilities|String|ToString(Text) _text))
  ;[1 1 1] Backspace Button
  (Rendering|Components|TextRender|SetText _enteredcodetext (Utilities|Text|ToText(String) (Utilities|String|GetSubstring _returnvalue 0 (- (Utilities|String|Len _returnvalue) 1)))))

(event Custom|EnteredButton
  (params (Value :type Text) (IsConfirmed :type Boolean) (IsBackspaced :type Boolean))
  (bind _enteredcodetext (Variables|Default|GetEnteredCodeText))
  ;[1 1 1] Type Numbers
  (if IsConfirmed
    (CallFunction|Confirmed)
    (elif IsBackspaced
      (CallFunction|Backspace)
      (elif (Variables|Default|GetCanEnter)
        (Audio|PlaySound2D "/Game/Sounds/click-button.click-button" 1.0 1.0 0.0 0 0)
        (Rendering|Components|TextRender|SetText _enteredcodetext (Utilities|Text|ToText(String) (Utilities|String|Replace (Utilities|String|ToString(Text) (Variables|/Script/Engine.TextRenderComponent|GetText (Variables|Default|GetEnteredCodeText))) (Utilities|String|GetSubstring (Utilities|String|MakeLiteralString "____") 0 (Utilities|String|Len (Variables|Default|GetKeypadCode))))))
        (Rendering|Components|TextRender|SetText _enteredcodetext (Utilities|Text|ToText(String) (Utilities|String|Append (Utilities|String|ToString(Text) (Variables|/Script/Engine.TextRenderComponent|GetText (Variables|Default|GetEnteredCodeText))) (Utilities|String|ToString(Text) Value))))))))

(event Custom|Confirmed
  (bind _returnvalue (Game|GetPlayerController 0))
  (bind _returnvalue_2 (Game|GetPlayerController 0))
  (bind _enteredcodetext (Variables|Default|GetEnteredCodeText))
  (bind _enteredcodetext_2 (Variables|Default|GetEnteredCodeText))
  ;[1 1 1] Confirm Button
  (if (Utilities|Enum|Equal(Enum) (Variables|Default|GetKeypadCode) (Utilities|String|ToString(Text) (Variables|/Script/Engine.TextRenderComponent|GetText (Variables|Default|GetEnteredCodeText))))
    (Utilities|FlowControl|Sequence
      (:then_0
        ;;[1 1 1] If Code Is Correct
        (Rendering|Components|TextRender|SetText _enteredcodetext_2 (Utilities|Text|MakeLiteralText "Correct"))
        (Rendering|Components|TextRender|SetTextRenderColor _enteredcodetext_2 (Math|Color|MakeColor 255 0 0 255))
        (Rendering|Material|SetMaterial (Variables|Default|GetKeypad) 0 "/Game/Geometry/Meshes/CubeMaterial.CubeMaterial")
        (Utilities|FlowControl|RetriggerableDelay 2.0)
        (bind _output_get (Variables|/Script/Engine.PlayerController|SetbShowMouseCursor _returnvalue_2 false))
        (bind _output_get_2 (Variables|/Script/Engine.PlayerController|SetbEnableMouseOverEvents _returnvalue_2 _output_get))
        (Variables|/Script/Engine.PlayerController|SetbEnableClickEvents _returnvalue_2 _output_get_2)
        (for _array_element (Variables|Default|GetButtonArray)
          (bind _asbp_keypad_button (Utilities|Casting|CastToBP_KeypadButton (Variables|/Script/Engine.ChildActorComponent|GetChildActor _array_element)))
          (Default|ResetButtons _asbp_keypad_button))
        (CallFunction|ResetCameraInteractionAnytime)
        (Components|DestroyComponent (Variables|Default|GetCollision))
        (bind _returnvalue_3 (Actor|GetActorOfClass "/Game/ThirdPersonBP/Blueprints/Interfaces/Interactables/BP_LockedBox.BP_LockedBox_C"))
        (Variables|/Game/ThirdPersonBP/Blueprints/Interfaces/Interactables/BP_LockedBox.BP_LockedBox_C|SetCanOpen _returnvalue_3 true))
      (:then_1
        (Variables|Default|SetCanEnter false)
        (Audio|PlaySound2D 0 1.0 1.0 0.0 0 0)
        (Variables|Default|SetIsCorrect true))
      (:then_2
        (bind _returnvalue_4 (Actor|GetActorOfClass "/Game/ThirdPersonBP/Blueprints/Interfaces/Interactables/BP_Door.BP_Door_C"))
        (Variables|/Game/ThirdPersonBP/Blueprints/Interfaces/Interactables/BP_Door.BP_Door_C|SetCanOpen _returnvalue_4 true)))
    (else
      (Utilities|FlowControl|Sequence
        (:then_0
          ;;[1 1 1] If Code Is Wrong
          (Rendering|Components|TextRender|SetText _enteredcodetext (Utilities|Text|MakeLiteralText "Wrong"))
          (Rendering|Components|TextRender|SetTextRenderColor _enteredcodetext (Math|Color|MakeColor 0 0 255 255))
          (Rendering|Material|SetMaterial (Variables|Default|GetKeypad) 0 "/Game/Geometry/Meshes/CubeMaterial.CubeMaterial")
          (Utilities|FlowControl|RetriggerableDelay 2.0)
          (bind _output_get_3 (Variables|/Script/Engine.PlayerController|SetbEnableMouseOverEvents _returnvalue false))
          (Variables|/Script/Engine.PlayerController|SetbEnableClickEvents _returnvalue _output_get_3)
          (for _array_element_2 (Variables|Default|GetButtonArray)
            (bind _asbp_keypad_button_2 (Utilities|Casting|CastToBP_KeypadButton (Variables|/Script/Engine.ChildActorComponent|GetChildActor _array_element_2)))
            (Default|ResetButtons _asbp_keypad_button_2))
          (CallFunction|Initiate)
          (Variables|Default|SetCanEnter true))
        (:then_1
          (Variables|Default|SetCanEnter false)
          (Audio|PlaySound2D 0 1.0 1.0 0.0 0 0))))))

(event Custom|Reset%20Camera%20Interaction%20Anytime
  (bind _returnvalue (Game|GetPlayerController 0))
  ;[1 1 1] Confirm Button
  (Variables|/Game/ThirdPersonBP/Blueprints/ThirdPersonCharacter.ThirdPersonCharacter_C|SetCurrentPlayerState (Variables|Default|GetPlayerRef) "NewEnumerator0")
  (Game|Player|SetViewTargetwithBlend (Game|GetPlayerController 0) (Components|GetOwner (Variables|/Game/ThirdPersonBP/Blueprints/ThirdPersonCharacter.ThirdPersonCharacter_C|GetFollowCamera (.AsThird%20Person%20Character (Utilities|Casting|CastToThirdPersonCharacter (Game|Player|GetPlayerPawn 0))))) 0.4 "VTBlend_Linear" 0.0 false)
  (Rendering|Components|TextRender|SetText (Variables|Default|GetEnteredCodeText) (Utilities|Text|MakeLiteralText ""))
  (bind _output_get (Variables|/Script/Engine.PlayerController|SetbShowMouseCursor _returnvalue false))
  (bind _output_get_2 (Variables|/Script/Engine.PlayerController|SetbEnableMouseOverEvents _returnvalue _output_get))
  (Variables|/Script/Engine.PlayerController|SetbEnableClickEvents _returnvalue _output_get_2)
  (Variables|Default|SetCanEnter true))

(event EventBeginPlay
  (bind _asthird_person_character (Utilities|Casting|CastToThirdPersonCharacter (Game|GetPlayerCharacter 0)))
  (Variables|Default|SetPlayerRef _asthird_person_character))

(event EventInteraction
  (params (CallingActor :type Actor%20Object%20Reference))
  ;[1 1 1] Interface Interaction
  (if (not (Variables|Default|GetIsCorrect))
    (switch Utilities|FlowControl|Switch|SwitchonE_PlayerState (Variables|/Game/ThirdPersonBP/Blueprints/ThirdPersonCharacter.ThirdPersonCharacter_C|GetCurrentPlayerState (Variables|Default|GetPlayerRef))
      (:NewEnumerator0
        (CallFunction|OnInteracted)
        (Variables|/Game/ThirdPersonBP/Blueprints/ThirdPersonCharacter.ThirdPersonCharacter_C|SetKeypadInteraction (Variables|Default|GetPlayerRef) self)))))

(fn ConstructionScript)